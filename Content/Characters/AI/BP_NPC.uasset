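; BP_NPC is an enemy NPC that takes lives from the player character on contact and triggers the game-over screen.
; Beginning an overlap starts a one-second delay, then raises an attacking flag for three seconds and removes one life if contact is still flagged.
; At zero lives it plays music, pauses the game, shows the Lose_HUD widget and mouse cursor, and sets game-only input.
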(event `self.ReceiveActorEndOverlap`
  (params (OtherActor :type "Actor Object Reference"))
  (cast `/Game/ThirdPerson/Blueprints/BP_ThirdPersonCharacter` OtherActor)
  (set `self.IsToutching` false))

(event `self.ReceiveActorBeginOverlap`
  (params (OtherActor :type "Actor Object Reference"))
  (bind _returnvalue (`GameplayStatics.GetPlayerController` 0))
  (bind _asbp_third_person_character (cast `/Game/ThirdPerson/Blueprints/BP_ThirdPersonCharacter` OtherActor))
  (set `self.IsToutching` true)
  (`KismetSystemLibrary.Delay` 1.0)
  (`self.Attack`)
  (if (`self.IsToutching`)
    (bind _result (`/Engine/EditorBlueprintResources/StandardMacros.DecrementInt` (`/Game/ThirdPerson/Blueprints/BP_ThirdPersonCharacter.nbrvie` _asbp_third_person_character))
      (:`  `
        (if (not (> _result 0))
          (`GameplayStatics.PlaySound2D` "/Game/FX/Amnesia__The_Dark_Descent_Soundtrack_-_Main_Menu__extended__1_.Amnesia__The_Dark_Descent_Soundtrack_-_Main_Menu__extended__1_" 1.0 1.0 0.0 null null)
          (`GameplayStatics.SetGamePaused` true)
          (bind _returnvalue_2 (`|CreateWidget` "/Game/HUD/lose_HUD.lose_HUD_C"))
          (`UserWidget.AddToViewport` _returnvalue_2 0)
          (set `PlayerController.bShowMouseCursor` true _returnvalue)
          (`WidgetBlueprintLibrary.SetInputMode_GameOnly` _returnvalue))))))

(event `Attack`
  (set `self.isAttacking` true)
  (`KismetSystemLibrary.Delay` 3.0)
  (set `self.isAttacking` false))

(fn `UserConstructionScript`)
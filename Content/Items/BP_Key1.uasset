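; BP_Key1 is a key item actor that spins and bobs in the level.
; A pair of timelines, one played forward and one in reverse, trigger each other to loop the sphere's vertical motion, while Tick applies constant yaw rotation.
; The overlap event is empty: the pickup logic that updates the character's escape item count or CanEscape and destroys the key is disconnected and never runs.
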(event `self.ReceiveActorBeginOverlap`
  (params (OtherActor :type "Actor Object Reference"))
  ;[1 1 1] PickUp
)

(event `self.ReceiveBeginPlay`
  (bind _sphere (`self.Sphere`))
  ;[1 1 1] Floating
  (bind (_direction _z_axis_pos) (`Timeline|Timeline` :!label _label)
    (:`Update`
      (`SceneComponent.K2_SetRelativeLocation` _sphere _z_axis_pos false false))
    (:`Finished`
      (bind (_direction_2 _z_axis_pos_2) (`Timeline|Timeline_0` :!via `ReverseFromEnd`)
        (:`Update`
          (`SceneComponent.K2_SetRelativeLocation` _sphere _z_axis_pos_2 false false))
        (:`Finished`
          (goto _label :!via `PlayFromStart`))))))

(event `self.ReceiveTick`
  (params (DeltaSeconds :type "Float (single-precision)"))
  ;[1 1 1] Rotation
  (`self.K2_AddActorLocalRotation` (`KismetMathLibrary.MakeRotator` 0.0 0.0 (* DeltaSeconds 50.0))))

(fn `UserConstructionScript`)
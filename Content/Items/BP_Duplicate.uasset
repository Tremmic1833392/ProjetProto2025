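; BP_Duplicate is a floating pickup that duplicates the player when touched.
; On overlap with a BP_ThirdPersonCharacter, it spawns another character of that class at the same transform, then destroys itself.
; From BeginPlay, two timelines alternate in an endless loop to bob the Cube along Z, one playing forward and the other in reverse.
; Tick spins the actor around yaw at a constant, frame-rate-independent speed.
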(event `self.ReceiveActorBeginOverlap`
  (params (OtherActor :type "Actor Object Reference"))
  ;[1 1 1] Duplicate Player
  (bind _asbp_third_person_character (cast `/Game/ThirdPerson/Blueprints/BP_ThirdPersonCharacter` OtherActor))
  (`|SpawnActorFromClass` "/Game/ThirdPerson/Blueprints/BP_ThirdPersonCharacter.BP_ThirdPersonCharacter_C" (`self.GetTransform` _asbp_third_person_character) "Undefined" "MultiplyWithRoot" null null)
  (`self.K2_DestroyActor`))

(event `self.ReceiveBeginPlay`
  ;[1 1 1] Floating
  (bind (_direction _z_axis_pos) (`Timeline|Floating` :!label _label)
    (:`Update`
      (`SceneComponent.K2_SetRelativeLocation` (`self.Cube`) _z_axis_pos false false))
    (:`Finished`
      (bind (_direction_2 _z_axis_pos_2) (`Timeline|Timeline` :!via `ReverseFromEnd`)
        (:`Update`
          (`SceneComponent.K2_SetRelativeLocation` (`self.Cube`) _z_axis_pos_2 false false))
        (:`Finished`
          (goto _label :!via `PlayFromStart`))))))

(event `self.ReceiveTick`
  (params (DeltaSeconds :type "Float (single-precision)"))
  ;[1 1 1] Rotation
  (`self.K2_AddActorLocalRotation` (`KismetMathLibrary.MakeRotator` 0.0 0.0 (* DeltaSeconds 50.0))))

(fn `UserConstructionScript`)